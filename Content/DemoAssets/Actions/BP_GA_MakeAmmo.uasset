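; GOAP action that sends an AI character to an ammo generation target to gain ammo.
; UpdateCost queues an asynchronous EQS query, then on later calls stores the result as the target and derives cost from its distance.
; Execute tints the character and walks it to the target, then adds ammo and sets GOAP state once in range.
; The target is not destroyed, despite the inline comment.
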(event `self.UpdateCost`
  (params (controller :type "GOAPAIController Object Reference"))
  (bind _returnvalue (`Actor.K2_GetActorLocation` (`Controller.K2_GetPawn` controller)))
  (bind _output (`|GetArrayItem` (`self.QueryResultsActor`)))
  (bind _returnvalue_2 (`Actor.K2_GetActorLocation` _output))
  ;[1 1 1] IF we don't have a target (ammo box), run the EQS query for one and wait until results return
  (if (`self.IsEQSQueryRequestPending`)
    (if (`self.IsEQSResultsAvailable`)
      (`/Engine/EditorBlueprintResources/StandardMacros.IsValid` _output
        (:`Is Valid`
          (set `self.ActionTarget` _output)
          (`KismetSystemLibrary.DrawDebugLine` controller _returnvalue _returnvalue_2 (struct :`R` 0.94 :`G` 0.086832 :`B` 0.913466 :`A` 1.0) 1.0 3.0)
          (set `self.Cost` (`KismetMathLibrary.FTrunc` (* (`KismetMathLibrary.VSize` (- _returnvalue_2 _returnvalue)) 0.02))))
        (:`Is Not Valid`
          _))
      (set `self.IsEQSQueryRequestPending` false)
      (set `self.IsEQSResultsAvailable` false))
    (else
      (`GOAPAIController.AddEQSJob` controller self "/GOAPer/DemoAssets/Actions/BP_EQS_Ammo_Gen_Query.BP_EQS_Ammo_Gen_Query" "SingleResult")
      (set `self.IsEQSQueryRequestPending` true)
      (set `self.IsEQSResultsAvailable` false))))

(fn `Execute`
  (params (controller :type "GOAPAIController Object Reference") (DeltaSeconds :type "Float (double-precision)"))
  (returns (ReturnValue :type Boolean))
  (`|ExecutionSequence`
    (:`then_0`
      ;[1 1 1] Comment
      (if (`KismetSystemLibrary.IsValid` (`self.ActionTarget`))
        (bind _asbp_goap_character (cast `/GOAPer/DemoAssets/BP_GOAP_Character` (`Controller.K2_GetPawn` controller)))
        (`/GOAPer/DemoAssets/BP_GOAP_Character.SetColor` _asbp_goap_character (1.0 0.0 1.0))
        (`AIController.K2_ClearFocus` controller)
        (else
          (return false))))
    (:`then_1`
      ;[1 1 1] Move towards it if we're out of range
      (if (`self.IsInRange` controller)
        ;[1 1 1] If we're in range, destroy it and finish
        (bind _asbp_goap_character_2 (cast `/GOAPer/DemoAssets/BP_GOAP_Character` (`Controller.K2_GetPawn` controller)))
        (set `/GOAPer/DemoAssets/BP_GOAP_Character.AmmoCount` (+ (`/GOAPer/DemoAssets/BP_GOAP_Character.AmmoCount` _asbp_goap_character_2) 10) _asbp_goap_character_2)
        (`GOAPAIController.SetGOAPState` controller (struct :`Key` 2) true)
        (return true)
        (else
          (bind _returnvalue (`GOAPAIController.IsMoveCompleted` controller))
          (if _returnvalue
            (`GOAPAIController.SetMoveToStateWithTarget` controller (`self.ActionTarget`) (- (`self.InteractionRange`) 200.0) 200.0))
          (return false))))))