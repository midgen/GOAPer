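; GOAP action that sends an AI character running to a cover location.
; UpdateCost queues a single-result EQS cover query, polls for results, then stores the location and sets cost from straight-line distance in meters.
; Execute tints the character, clears focus and requests the move, then resets the target to a below -100 Z sentinel.
; While that sentinel holds, it waits for move completion, then sets the GOAP state and succeeds.
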(event `self.UpdateCost`
  (params (controller :type "GOAPAIController Object Reference"))
  (bind _returnvalue (`Actor.K2_GetActorLocation` (`Controller.K2_GetPawn` controller)))
  (bind _output (`|GetArrayItem` (`self.QueryResultsLocation`)))
  ;[1 1 1] IF we don't have a target (ammo box), run the EQS query for one and wait until results return
  (if (`self.IsEQSQueryRequestPending`)
    (if (`self.IsEQSResultsAvailable`)
      (bind _output_get (set `self.MoveToTarget` _output))
      (`KismetSystemLibrary.DrawDebugLine` controller _returnvalue _output_get (struct :`R` 0.042307 :`G` 0.94 :`A` 1.0) 1.0 3.0)
      (set `self.Cost` (`KismetMathLibrary.FTrunc` (* (`KismetMathLibrary.VSize` (- _output _returnvalue)) 0.01)))
      (set `self.IsEQSQueryRequestPending` false)
      (set `self.IsEQSResultsAvailable` false))
    (else
      (`GOAPAIController.AddEQSJob` controller self "/GOAPer/DemoAssets/Actions/BP_EQS_Cover_Query.BP_EQS_Cover_Query" "SingleResult")
      (set `self.IsEQSQueryRequestPending` true)
      (set `self.IsEQSResultsAvailable` false)
      (set `self.MoveToTarget` (0.0 0.0 -200.0)))))

(fn `Execute`
  (params (controller :type "GOAPAIController Object Reference") (DeltaSeconds :type "Float (double-precision)"))
  (returns (ReturnValue :type Boolean))
  (`|ExecutionSequence`
    (:`then_0`
      ;[1 1 1] Comment
      (bind _asbp_goap_character (cast `/GOAPer/DemoAssets/BP_GOAP_Character` (`Controller.K2_GetPawn` controller)))
      (`/GOAPer/DemoAssets/BP_GOAP_Character.SetColor` _asbp_goap_character (0.8 0.3 0.0))
      (`AIController.K2_ClearFocus` controller))
    (:`then_1`
      ;[1 1 1] See if we have a valid move target
      (if (< (.z (`self.MoveToTarget`)) -100.0)
        ;[1 1 1] Move completed
        (bind _returnvalue (`GOAPAIController.IsMoveCompleted` controller))
        (if _returnvalue
          (`GOAPAIController.SetGOAPState` :`self` controller :`Value` true)
          (return true)
          (else
            (return false)))
        (else
          ;[1 1 1] When the query finishes, request the move!
          (`GOAPAIController.SetMoveToStateWithLocation` controller (`self.MoveToTarget`) 450.0)
          (set `self.MoveToTarget` (0.0 0.0 -200.0))
          (return false))))))