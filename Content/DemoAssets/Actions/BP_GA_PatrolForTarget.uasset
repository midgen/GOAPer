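; GOAP action that makes an AI pawn patrol at random until it has a target.
; Execute succeeds once the controller has a valid focus actor, stopping movement and setting the GOAP state to true.
; Until then it returns false, and whenever the previous move completes it walks the pawn to a random navigable point around its location and tints the GOAP character blue.
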(fn `Execute`
  (params (controller :type "GOAPAIController Object Reference") (DeltaSeconds :type "Float (double-precision)"))
  (returns (ReturnValue :type Boolean))
  (bind _returnvalue (`Controller.K2_GetPawn` controller))
  (`|ExecutionSequence`
    (:`then_0`
      ;[1 1 1] Complete if we already have a valid target
      (`/Engine/EditorBlueprintResources/StandardMacros.IsValid` (`AIController.GetFocusActor` controller)
        (:`Is Valid`
          (`Controller.StopMovement` controller)
          (`GOAPAIController.SetGOAPState` controller (struct :`Key` 3) true)
          (return true))))
    (:`then_1`
      (bind _returnvalue_2 (`GOAPAIController.IsMoveCompleted` controller))
      (if _returnvalue_2
        ;[1 1 1] Otherwise, pick a random point
        (`GOAPAIController.SetMoveToStateWithLocation` controller (`NavigationSystemV1.K2_GetRandomLocationInNavigableRadius` _returnvalue (`Actor.K2_GetActorLocation` _returnvalue) 2000.0 null null) 200.0)
        (bind _asbp_goap_character (cast `/GOAPer/DemoAssets/BP_GOAP_Character` (`Controller.K2_GetPawn` controller)))
        (`/GOAPer/DemoAssets/BP_GOAP_Character.SetColor` _asbp_goap_character (0.0 0.4 0.8))
        (return false)
        (else
          (return false))))))