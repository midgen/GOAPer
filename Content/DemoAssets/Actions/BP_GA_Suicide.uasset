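; GOAP action that makes an AI agent close on its focus actor and blow up, destroying both the target and itself.
; Cost scales with distance to the focus actor, with a debug line drawn to it, and falls back to a fixed value without one.
; Execute tints the pawn white, moves it toward the target until in range, then spawns an emitter and destroys both actors.
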(event `self.UpdateCost`
  (params (controller :type "GOAPAIController Object Reference"))
  (bind _returnvalue (`AIController.GetFocusActor` controller))
  (bind _returnvalue_2 (`Actor.K2_GetActorLocation` _returnvalue))
  (bind _returnvalue_3 (`Actor.K2_GetActorLocation` (`Controller.K2_GetPawn` controller)))
  ;[1 1 1] IF we don't have a target (ammo box), run the EQS query for one and wait until results return
  (`/Engine/EditorBlueprintResources/StandardMacros.IsValid` _returnvalue
    (:`Is Valid`
      (`KismetSystemLibrary.DrawDebugLine` controller _returnvalue_3 _returnvalue_2 (struct :`R` 1.0 :`B` 0.190264 :`A` 1.0) 1.0 3.0)
      (set `self.Cost` (`KismetMathLibrary.FTrunc` (* (`KismetMathLibrary.VSize` (- _returnvalue_2 _returnvalue_3)) 0.03))))
    (:`Is Not Valid`
      (set `self.Cost` 100))))

(fn `Execute`
  (params (controller :type "GOAPAIController Object Reference") (DeltaSeconds :type "Float (double-precision)"))
  (returns (ReturnValue :type Boolean))
  (bind _returnvalue (`AIController.GetFocusActor` controller))
  (`|ExecutionSequence`
    (:`then_0`
      (bind _asbp_goap_character (cast `/GOAPer/DemoAssets/BP_GOAP_Character` (`Controller.K2_GetPawn` controller)))
      (`/GOAPer/DemoAssets/BP_GOAP_Character.SetColor` _asbp_goap_character (1.0 1.0 1.0)))
    (:`then_1`
      (`/Engine/EditorBlueprintResources/StandardMacros.IsValid` _returnvalue
        (:`Is Valid`
          (set `self.ActionTarget` _returnvalue)
          (if (`self.IsInRange` controller)
            ;[1 1 1] Destroy the target and self
            (`GameplayStatics.SpawnEmitterAtLocation` controller null (`Actor.K2_GetActorLocation` (`Controller.K2_GetPawn` controller)))
            (`Actor.K2_DestroyActor` (`self.ActionTarget`))
            (`Actor.K2_DestroyActor` (`Controller.K2_GetPawn` controller))
            (return true)
            (else
              ;[1 1 1] Move towards it if we're out of range
              (`GOAPAIController.SetMoveToStateWithTarget` controller (`self.ActionTarget`) (- (`self.InteractionRange`) 200.0) 400.0)
              (return false))))))))