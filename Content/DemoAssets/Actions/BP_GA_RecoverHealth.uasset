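; GOAP action that lets an AI-controlled BP_GOAP_Character regenerate health over time.
; Execute returns done if its effects are already satisfied; otherwise it tints the pawn green and raises HP at a fixed per-second rate until full.
; At full health it sets a GOAP state true and a goal false on the controller, then clears the current action and plan.
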(fn `Execute`
  (params (controller :type "GOAPAIController Object Reference") (DeltaSeconds :type "Float (double-precision)"))
  (returns (ReturnValue :type Boolean))
  (locals (RegenRate :type Boolean))
  (if (`self.AreEffectsSatisfied` controller)
    (return true)
    (else
      (bind _asbp_goap_character (cast `/GOAPer/DemoAssets/BP_GOAP_Character` (`Controller.K2_GetPawn` controller)))
      (`/GOAPer/DemoAssets/BP_GOAP_Character.SetColor` _asbp_goap_character (0.0 1.0 0.0))
      (if (< (`/GOAPer/DemoAssets/BP_GOAP_Character.HP` _asbp_goap_character) 100.0)
        (set `/GOAPer/DemoAssets/BP_GOAP_Character.HP` (+ (`/GOAPer/DemoAssets/BP_GOAP_Character.HP` _asbp_goap_character) (* DeltaSeconds 20.0)) _asbp_goap_character)
        (return false)
        (else
          (`GOAPAIController.SetGOAPState` controller (struct :`Key` 4) true)
          (`GOAPAIController.SetGOAPGoal` controller (struct :`Key` 5) false)
          (`GOAPAIController.ClearCurrentActionAndPlan` controller)
          (return true))))))