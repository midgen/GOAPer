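; GOAP action for a secondary attack, in which an AI pawn fires at its controller's focus actor.
; UpdateCost scales with target distance, at a cheaper rate inside InteractionRange, and uses a fixed fallback without a valid focus.
; Execute tints the character red, caches the AI controller, then yaws toward the target and calls Fire, staying unfinished until the focus is invalid.
; It then updates GOAP state and reports completion.
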(event `self.UpdateCost`
  (params (controller :type "GOAPAIController Object Reference"))
  (bind _returnvalue (`AIController.GetFocusActor` controller))
  (bind _returnvalue_2 (`KismetMathLibrary.VSize` (- (`Actor.K2_GetActorLocation` _returnvalue) (`Actor.K2_GetActorLocation` (`Controller.K2_GetPawn` controller)))))
  (`/Engine/EditorBlueprintResources/StandardMacros.IsValid` _returnvalue
    (:`Is Valid`
      (if (< _returnvalue_2 (`self.InteractionRange`))
        (set `self.Cost` (`KismetMathLibrary.FTrunc` (* _returnvalue_2 0.005)))
        (else
          (set `self.Cost` (`KismetMathLibrary.FTrunc` (* _returnvalue_2 0.01))))))
    (:`Is Not Valid`
      (set `self.Cost` 100))))

(fn `Execute`
  (params (controller :type "GOAPAIController Object Reference") (DeltaSeconds :type "Float (double-precision)"))
  (returns (ReturnValue :type Boolean))
  (bind _returnvalue (`Controller.K2_GetPawn` controller))
  (bind _returnvalue_2 (`AIController.GetFocusActor` controller))
  (bind _bp_ai_controllerref (`self.BP_AI_ControllerRef`))
  (`|ExecutionSequence`
    (:`then_0`
      (bind _asbp_goap_character (cast `/GOAPer/DemoAssets/BP_GOAP_Character` (`Controller.K2_GetPawn` controller)))
      (`/GOAPer/DemoAssets/BP_GOAP_Character.SetColor` _asbp_goap_character (0.5 0.0 0.0)))
    (:`then_1`
      ;[1 1 1] First cast and set our controller ref if not done already
      (if (not (`KismetSystemLibrary.IsValid` _bp_ai_controllerref))
        (bind _asbp_goap_ai_controller (cast `/GOAPer/DemoAssets/BP_GOAP_AI_Controller` controller)
          (:`then`
            (set `self.BP_AI_ControllerRef` _asbp_goap_ai_controller))
          (:`CastFailed`
            (return false)))))
    (:`then_2`
      ;[1 1 1] Target is dead, complete the action
      (`/Engine/EditorBlueprintResources/StandardMacros.IsValid` _returnvalue_2
        (:`Is Valid`
          ;[1 1 1] Do the attacking here
          (`Actor.K2_SetActorRotation` _returnvalue (`KismetMathLibrary.MakeRotator` 0.0 0.0 (.yaw (`KismetMathLibrary.FindLookAtRotation` (`Actor.K2_GetActorLocation` _returnvalue) (`Actor.K2_GetActorLocation` _returnvalue_2)))) false)
          (bind _asbp_goap_character_2 (cast `/GOAPer/DemoAssets/BP_GOAP_Character` (`Controller.K2_GetPawn` controller))
            (:`then`
              (`/GOAPer/DemoAssets/BP_GOAP_Character.Fire` _asbp_goap_character_2))
            (:`CastFailed`
              _))
          (return false))
        (:`Is Not Valid`
          (`GOAPAIController.SetGOAPState` _bp_ai_controllerref (struct :`Key` 5) true)
          (`GOAPAIController.SetGOAPState` _bp_ai_controllerref (struct :`Key` 3) false)
          (return true))))))