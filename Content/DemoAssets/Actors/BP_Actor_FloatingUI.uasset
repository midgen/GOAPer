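; Floating status UI actor that hovers above the pawn of a given controller and hosts a BP_Status_Widget.
; SetRefs stores the controller and character references and forwards both to the widget.
; Each Tick it snaps to just above the controlled pawn and eases its rotation toward the direction from that pawn to player 0's pawn, using delta time as the lerp alpha.
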(event `self.ReceiveTick`
  (params (DeltaSeconds :type "Float (single-precision)"))
  (bind _returnvalue (`self.K2_GetActorLocation` (`Controller.K2_GetPawn` (`self.ControllerRef`))))
  (`self.K2_SetActorLocation` (+ _returnvalue (0.0 0.0 50.0)))
  (`self.K2_SetActorRotation` (`KismetMathLibrary.RLerp` (`self.K2_GetActorRotation`) (`KismetMathLibrary.FindLookAtRotation` _returnvalue (`self.K2_GetActorLocation` (`GameplayStatics.GetPlayerPawn` 0))) DeltaSeconds)))

(fn `SetRefs`
  (params (ControllerREf :type "/GOAPer/DemoAssets/BP_GOAP_AI_Controller Object Reference") (CharacterRef :type "/GOAPer/DemoAssets/BP_GOAP_Character Object Reference"))
  (set `self.CharRef` CharacterRef)
  (set `self.ControllerRef` ControllerREf)
  (bind _asbp_status_widget (cast `/GOAPer/DemoAssets/UI/BP_Status_Widget` (`WidgetComponent.GetUserWidgetObject` (`self.Widget`))))
  (set `/GOAPer/DemoAssets/UI/BP_Status_Widget.CharacterRef` CharacterRef _asbp_status_widget)
  (set `/GOAPer/DemoAssets/UI/BP_Status_Widget.ControllerRef` ControllerREf _asbp_status_widget))

(fn `UserConstructionScript`)