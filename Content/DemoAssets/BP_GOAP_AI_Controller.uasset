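; GOAP AI controller that keeps world state and goals in sync with what its BP_GOAP_Character pawn perceives and needs.
; Tick updates target, pawn ammo and pickup availability states, polling all ammo pickups each frame, and sets a goal and clears the plan on low health.
; It drops unperceived focus actors and focuses the nearest sighted character or newly perceived ones, only when the current action allows interruption, stopping movement and replanning.
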(event `self.ReceiveBeginPlay`)

(event `self.ReceiveTick`
  (params (DeltaSeconds :type "Float (single-precision)"))
  (bind _returnvalue (`self.GetFocusActor`))
  (bind _returnvalue_2 (`KismetSystemLibrary.IsValid` (`self.GetFocusActor`)))
  (`|ExecutionSequence`
    (:`then_0`
      ;[1 1 1] Ensure 'HasTarget' state is correct
      (bind _returnvalue_3 (`self.GetGOAPState` (struct :`Key` 3)))
      (if _returnvalue_3
        (if (not _returnvalue_2)
          (`self.SetGOAPState` (struct :`Key` 3)))
        (elif _returnvalue_2
          (`self.SetGOAPState` (struct :`Key` 3) true))))
    (:`then_1`
      ;[1 1 1] Check if focus actor is still perceived
      (if (`KismetSystemLibrary.IsValid` _returnvalue)
        (set `self.IsFocusStillPerceived` false)
        (for _array_element (`AIPerceptionComponent.GetCurrentlyPerceivedActors` (`self.AIPerception`) null)
          (if (== _array_element _returnvalue)
            (set `self.IsFocusStillPerceived` true)
            (break)))
        (if (not (`self.IsFocusStillPerceived`))
          (`self.K2_SetFocus` null))))
    (:`then_2`
      ;[1 1 1] React to low health
      (bind _asbp_goap_character (cast `/GOAPer/DemoAssets/BP_GOAP_Character` (`self.K2_GetPawn`)))
      (if (< (`/GOAPer/DemoAssets/BP_GOAP_Character.HP` _asbp_goap_character) 50.0)
        (`self.SetGOAPState` (struct :`Key` 4))
        (bind _returnvalue_4 (`self.IsGoalSet` (struct :`Key` 4) true))
        (if (not _returnvalue_4)
          (`self.SetGOAPGoal` (struct :`Key` 4) true)
          (`self.ClearCurrentActionAndPlan`))))
    (:`then_3`
      ;[1 1 1] Evaluate HasAmmo state
      (`self.SetGOAPState` (struct :`Key` 2) (> (`/GOAPer/DemoAssets/BP_GOAP_Character.AmmoCount` _asbp_goap_character) 0)))
    (:`then_4`
      ;[1 1 1] Evaluate IsAmmoAvailable - THIS IS SUPER BAD CODE DO NOT JUDGE ME
      (bind _outactors (`GameplayStatics.GetAllActorsOfClass` "/GOAPer/DemoAssets/Actors/BP_Pickup_Ammo.BP_Pickup_Ammo_C"))
      (`self.SetGOAPState` (struct :`Key` 6) (> (`KismetArrayLibrary.Array_Length` _outactors) 0)))
    (:`then_5`
      ;[1 1 1] Check perceived actors here
      (`self.ProcessPerception`))))

(event `self.AIPerception.OnPerceptionUpdated`
  (params (UpdatedActors :type "Array of Actor Object Reference (by ref)"))
  (bind _returnvalue (`self.GetFocusActor`))
  ;[1 1 1] Perception
  (for _array_element UpdatedActors
    (if (`KismetSystemLibrary.IsValid` _returnvalue)
      (if (!= _returnvalue _array_element)
        (bind _shouldinterrupt (`self.CheckInterrupt` :!label _label))
        (if _shouldinterrupt
          (cast `/GOAPer/DemoAssets/BP_GOAP_Character` _array_element)
          (`self.K2_SetFocus` _array_element)
          (`self.SetGOAPState` (struct :`Key` 3) true)
          (break)))
      (else
        (goto _label)))))

(fn `CheckInterrupt`
  (returns (ShouldInterrupt :type Boolean))
  (bind _currentaction (`self.CurrentAction`))
  (`/Engine/EditorBlueprintResources/StandardMacros.IsValid` _currentaction
    (:`Is Valid`
      (if (`GOAPAction.ShouldInterruptMoveOnTargetAcquisition` _currentaction)
        (`self.StopMovement`)
        (`self.ClearCurrentActionAndPlan`)
        (return true)
        (else
          _)))
    (:`Is Not Valid`
      _))
  (return false))

(fn `ProcessPerception`
  (locals (NearestActorDistance :type "Float (double-precision)") (NearestActorRef :type "Actor Object Reference") (WasAICharPerceived :type Boolean))
  (bind _output_get (set `local.NearestActorDistance` 100000.0))
  (set `local.WasAICharPerceived` false)
  (for _array_element (`AIPerceptionComponent.GetPerceivedActors` (`self.GetAIPerceptionComponent`) "/Script/AIModule.AISense_Sight")
    (bind _asbp_goap_character (cast `/GOAPer/DemoAssets/BP_GOAP_Character` _array_element))
    (bind _returnvalue (`KismetMathLibrary.VSize` (- (`self.K2_GetActorLocation` _asbp_goap_character) (`self.K2_GetActorLocation` (`self.K2_GetPawn`)))))
    (if (< _returnvalue _output_get)
      (set `local.NearestActorDistance` _returnvalue)
      (set `local.NearestActorRef` _array_element)
      (set `local.WasAICharPerceived` true)))
  (if (`local.WasAICharPerceived`)
    (bind _shouldinterrupt (`self.CheckInterrupt`))
    (if _shouldinterrupt
      (`self.K2_SetFocus` (`local.NearestActorRef`)))))

(fn `UserConstructionScript`)