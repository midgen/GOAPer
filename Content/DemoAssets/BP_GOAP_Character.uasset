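; Demo GOAP AI combat character with HP, ammo and two attacks sharing one cooldown and ammo check.
; Spawns a floating UI actor linked to its controller, destroyed alongside it.
; Damage lowers HP and clears a GOAP state on the controller; negative HP destroys the character.
; Fire spawns a projectile and spends ammo, while FireSecondary directly damages the focus actor with a debug cone, spending none.
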(event `self.ReceiveBeginPlay`
  (bind _returnvalue (`|SpawnActorFromClass` "/GOAPer/DemoAssets/Actors/BP_Actor_FloatingUI.BP_Actor_FloatingUI_C" (`KismetMathLibrary.MakeTransform` (+ (`self.K2_GetActorLocation`) (0.0 0.0 200.0))) "Undefined" "OverrideRootScale" null null))
  (set `self.StatusWidgetActor` _returnvalue)
  (bind _asbp_goap_ai_controller (cast `/GOAPer/DemoAssets/BP_GOAP_AI_Controller` (`AIBlueprintHelperLibrary.GetAIController` self)))
  (`/GOAPer/DemoAssets/Actors/BP_Actor_FloatingUI.SetRefs` _returnvalue _asbp_goap_ai_controller self))

(event `self.ReceiveAnyDamage`
  (params (Damage :type "Float (single-precision)") (DamageType :type "DamageType Object Reference") (InstigatedBy :type "Controller Object Reference") (DamageCauser :type "Actor Object Reference"))
  (bind _hp (`self.HP`))
  (set `self.HP` (- _hp Damage))
  (bind _asbp_goap_ai_controller (cast `/GOAPer/DemoAssets/BP_GOAP_AI_Controller` (`AIBlueprintHelperLibrary.GetAIController` self)))
  (`GOAPAIController.SetGOAPState` :`self` _asbp_goap_ai_controller)
  (if (< _hp 0.0) :!label _label
    (`self.K2_DestroyActor`)))

(event `self.ReceiveTick`
  (params (DeltaSeconds :type "Float (single-precision)"))
  (set `self.TimeSinceLastFire` (+ (`self.TimeSinceLastFire`) DeltaSeconds))
  (goto _label))

(event `self.ReceiveDestroyed`
  (`self.K2_DestroyActor` (`self.StatusWidgetActor`)))

(fn `Fire`
  (bind _returnvalue (`self.K2_GetActorRotation`))
  (if (and (> (`self.TimeSinceLastFire`) (`self.FireRate`)) (> (`self.AmmoCount`) 0))
    (set `self.TimeSinceLastFire` 0.0)
    (`|SpawnActorFromClass` "/GOAPer/DemoAssets/Actors/BP_Projectile.BP_Projectile_C" (`KismetMathLibrary.MakeTransform` (+ (`self.K2_GetActorLocation`) (* (`KismetMathLibrary.Normal` (`KismetMathLibrary.GetForwardVector` _returnvalue)) 60.0)) _returnvalue (0.1 0.1 0.1)) "AlwaysSpawn" "OverrideRootScale" null self)
    (set `self.AmmoCount` (- (`self.AmmoCount`) 1))))

(fn `FireSecondary`
  (bind _returnvalue (`self.K2_GetActorLocation`))
  (bind _returnvalue_2 (`AIController.GetFocusActor` (`AIBlueprintHelperLibrary.GetAIController` self)))
  (bind _returnvalue_3 (- (`self.K2_GetActorLocation` _returnvalue_2) _returnvalue))
  (if (and (> (`self.TimeSinceLastFire`) (`self.FireRate`)) (> (`self.AmmoCount`) 0))
    (set `self.TimeSinceLastFire` 0.0)
    (`KismetSystemLibrary.DrawDebugConeInDegrees` _returnvalue _returnvalue_3 (`KismetMathLibrary.VSize` _returnvalue_3) 5.0 5.0 12 (struct :`R` 1.0 :`G` 1.0 :`B` 1.0 :`A` 1.0) 0.5)
    (`GameplayStatics.ApplyDamage` _returnvalue_2 10.0 null self)))

(fn `SetColor`
  (params (NEwColor :type "Vector Structure"))
  (`MeshComponent.SetVectorParameterValueOnMaterials` (`self.Mesh`) "BodyColor" NEwColor))

(fn `UserConstructionScript`)